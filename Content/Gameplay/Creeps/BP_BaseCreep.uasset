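; BP_BaseCreep is a creep Blueprint, named as a base, that displays a colored, spinning cube.
; On BeginPlay it creates a dynamic material instance on the Cube and sets its Color parameter from CreepColor.
; Tick adds frame-rate-independent yaw, scaled so the cube turns RotationSpeed degrees every TimeToMakeRotate seconds.
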(event EventTick
  (params (DeltaSeconds :type Float%20%28single-precision%29))
  (Transformation|AddRelativeRotation (Variables|Default|GetCube) (Math|Rotator|MakeRotator 0.0 0.0 (/ (Variables|Default|GetRotationSpeed) (/ (Variables|Default|GetTimeToMakeRotate) DeltaSeconds))) false false))

(event EventBeginPlay
  (bind _returnvalue (Rendering|Material|CreateDynamicMaterialInstance (Variables|Default|GetCube) 0 0 "None" :!class /Script/Engine.PrimitiveComponent))
  (bind _output_get (Variables|Default|SetDynamic%20Material%20Instance _returnvalue))
  (Rendering|Material|SetVectorParameterValue _output_get "Color" (Variables|Default|GetCreepColor) :!class /Script/Engine.MaterialInstanceDynamic))

(fn ConstructionScript)