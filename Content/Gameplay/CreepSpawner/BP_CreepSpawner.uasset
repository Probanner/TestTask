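; BP_CreepSpawner is a spawn area actor that creates creeps around a sphere whose radius is set in the construction script.
; On BeginPlay it binds an event to the creep-spawned notification of the first BP_CreepSpawnController found.
; SpawnCreepByInfo looks up a creep row in DT_CreepsInfo and spawns its BP_BaseCreep class with the row's speed and color.
; GetRandomCoordinatesByRadius supplies the location, using random X/Y offsets within the sphere's scaled radius.
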(event EventBeginPlay
  (bind _outactors (Actor|GetAllActorsOfClass "/Game/Gameplay/SpawnController/BP_CreepSpawnController.BP_CreepSpawnController_C"))
  (EventDispatchers|BindEventtoCreepSpawned (Utilities|Array|Get(acopy) _outactors) (EventDispatchers|CreateEvent :!event SpawnCreepbyInfo)))

(event Collision|EventActorBeginOverlap
  (params (OtherActor :type Actor%20Object%20Reference)))

(event EventTick
  (params (DeltaSeconds :type Float%20%28single-precision%29)))

(fn ConstructionScript
  (Components|Sphere|SetSphereRadius (Variables|Default|GetShpere) (Variables|Default|GetRadius) true))

(fn SpawnCreepbyInfo
  (params (CreepName :type Name))
  (bind (_x _y _z) (Utilities|GetRandomCoordinatesbyRadius))
  (bind _returnvalue (Utilities|GetDataTableRow "/Game/Data/DT_CreepsInfo.DT_CreepsInfo" CreepName)
    (:then
      (bind _output_get (Variables|Default|SetCreepInfo _returnvalue))
      (bind _asbp_base_creep (Utilities|Casting|CastToBP_BaseCreepClass (.Class (Utilities|Struct|BreakS_CreepInfo _output_get))))
      (Game|SpawnActorfromClass _asbp_base_creep (Math|Transform|MakeTransform (Math|Vector|MakeVector _x _y _z) "0, 0, 0" "1,1,1") "AdjustIfPossibleButAlwaysSpawn" 0 (.Speed (Utilities|Struct|BreakS_CreepInfo _output_get)) (Math|Conversions|ToLinearColor(Color) (.TESTColor (Utilities|Struct|BreakS_CreepInfo _output_get))) (Variables|Default|GetTimeToMakeRotateInSec) 0))))